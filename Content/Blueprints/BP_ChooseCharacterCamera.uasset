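; Character-selection camera actor that steps a camera forward along spline points, each with its own look-at target.
; The construction script places and aims the camera at the start index.
; GoNext plays a timeline scaled by GoNextTime, lerping location straight between consecutive points and blending look-at rotations by the shortest path.
; The index advances when the timeline finishes, and GoNext does nothing at the last point.
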(event `self.ReceiveBeginPlay`
  (set `self.CurrentIndex` (`self.StartIndex`)))

(event `GoNext`
  (if (< (+ (`self.CurrentIndex`) 1) (`SplineComponent.GetNumberOfSplinePoints` (`self.Spline`)))
    (`TimelineComponent.SetPlayRate` (`self.ChangeLocation`) (/ 1.0 (`self.GoNextTime`)))
    (bind (_direction _newtrack_0) (`Timeline|ChangeLocation` :!via `PlayFromStart`)
      (:`Update`
        (`SceneComponent.K2_SetRelativeLocation` (`self.Camera`) (`KismetMathLibrary.VLerp` (`SplineComponent.GetLocationAtSplinePoint` (`self.Spline`) (`self.CurrentIndex`) "Local") (`SplineComponent.GetLocationAtSplinePoint` (`self.Spline`) (+ (`self.CurrentIndex`) 1) "Local") _newtrack_0) false false)
        (`SceneComponent.K2_SetRelativeRotation` (`self.Camera`) (`KismetMathLibrary.RLerp` (`KismetMathLibrary.FindLookAtRotation` (`SceneComponent.RelativeLocation` (`self.Camera`)) (`|GetArrayItem` (`self.LookAt`) (`self.CurrentIndex`))) (`KismetMathLibrary.FindLookAtRotation` (`SceneComponent.RelativeLocation` (`self.Camera`)) (`|GetArrayItem` (`self.LookAt`) (+ (`self.CurrentIndex`) 1))) _newtrack_0 true) false false))
      (:`Finished`
        (`/Engine/EditorBlueprintResources/StandardMacros.IncrementInt` (`self.CurrentIndex`))))))

(fn `UserConstructionScript`
  (bind _spline (`self.Spline`))
  (if (<= (`self.StartIndex`) (`SplineComponent.GetNumberOfSplinePoints` (`self.Spline`)))
    (`SceneComponent.K2_SetRelativeLocation` (`self.Camera`) (+ (`SceneComponent.RelativeLocation` _spline) (`SplineComponent.GetLocationAtSplinePoint` _spline (`self.StartIndex`) "Local")) false false)
    (if (`KismetArrayLibrary.Array_IsValidIndex` (`self.LookAt`) (`self.StartIndex`))
      (`SceneComponent.K2_SetRelativeRotation` (`self.Camera`) (`KismetMathLibrary.FindLookAtRotation` (`SceneComponent.RelativeLocation` (`self.Camera`)) (`|GetArrayItem` (`self.LookAt`) (`self.StartIndex`))) false false))))