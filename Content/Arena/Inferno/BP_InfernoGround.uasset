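; BP_InfernoGround is an Inferno arena ground actor that builds chains along four splines in its construction script.
; MakeChain divides each spline into SectionLength steps and adds a spline mesh component with the chain mesh per step, matching the spline's relative transform.
; Each segment starts InterlockLength early so neighboring links overlap, and its tangents are clamped to SectionLength.
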(fn `MakeChain`
  (params (Target :type "SplineComponent Object Reference") (StaticMesh :type "StaticMesh Object Reference"))
  (for _index (range (+ (`KismetMathLibrary.FTrunc` (/ (`SplineComponent.GetSplineLength` Target) (`self.SectionLength`))) 1))
    (bind _returnvalue (`AddComponent|NODE_AddSplineMeshComponent-0` :`RelativeTransform` (`KismetMathLibrary.MakeTransform` (`SceneComponent.RelativeLocation` Target) (`SceneComponent.RelativeRotation` Target) (`SceneComponent.RelativeScale3D` Target))))
    (`StaticMeshComponent.SetStaticMesh` _returnvalue StaticMesh)
    (`SplineMeshComponent.SetForwardAxis` _returnvalue "X" true)
    (bind _returnvalue_2 (- (* _index (`self.SectionLength`)) (`self.InterlockLength`)))
    (bind _returnvalue_3 (* (+ _index 1) (`self.SectionLength`)))
    (`SplineMeshComponent.SetStartAndEnd` _returnvalue (`SplineComponent.GetLocationAtDistanceAlongSpline` Target _returnvalue_2 "Local") (`KismetMathLibrary.ClampVectorSize` (`SplineComponent.GetTangentAtDistanceAlongSpline` Target _returnvalue_2 "Local") 0.0 (`self.SectionLength`)) (`SplineComponent.GetLocationAtDistanceAlongSpline` Target _returnvalue_3 "Local") (`KismetMathLibrary.ClampVectorSize` (`SplineComponent.GetTangentAtDistanceAlongSpline` Target _returnvalue_3 "Local") 0.0 (`self.SectionLength`)) true))
  (return))

(fn `UserConstructionScript`
  (`self.MakeChain` (`self.Spline`) "/Game/Enviroment/SplineMesh/Chain/S_Chain.S_Chain")
  (`self.MakeChain` (`self.Spline1`) "/Game/Enviroment/SplineMesh/Chain/S_Chain.S_Chain")
  (`self.MakeChain` (`self.Spline2`) "/Game/Enviroment/SplineMesh/Chain/S_Chain.S_Chain")
  (`self.MakeChain` (`self.Spline3`) "/Game/Enviroment/SplineMesh/Chain/S_Chain.S_Chain"))