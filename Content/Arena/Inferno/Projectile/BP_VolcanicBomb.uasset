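; BP_VolcanicBomb is a projectile in the Inferno arena that breaks destructible actors on contact.
; On firing, it reveals its Niagara effect and spawns an explosion at its location.
; Its trigger sphere applies damage and a velocity-directed impulse to overlapped DestructibleActors not already being destroyed.
; It then spawns another explosion, destroys the target's attach parent if valid, and destroys itself.
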(event `self.TriggerSphere.OnComponentBeginOverlap`
  (params (OverlappedComponent :type "PrimitiveComponent Object Reference") (OtherActor :type "Actor Object Reference") (OtherComp :type "PrimitiveComponent Object Reference") (OtherBodyIndex :type Integer) (bFromSweep :type Boolean) (SweepResult :type "HitResult Structure (by ref)"))
  (bind _asdestructible_actor (cast `DestructibleActor` OtherActor))
  (bind _destructiblecomponent (`DestructibleActor.DestructibleComponent` _asdestructible_actor))
  (if (not (`ActorComponent.IsBeingDestroyed` _destructiblecomponent))
    (`DestructibleComponent.ApplyDamage` _destructiblecomponent 50.0 (`self.K2_GetActorLocation`) (`self.GetVelocity`) 500.0)
    (`NiagaraFunctionLibrary.SpawnSystemAtLocation` "/Game/Effects/Particles/Explotion/NS_ky_explosion3.NS_ky_explosion3" (`self.K2_GetActorLocation`))
    (bind _returnvalue (`self.GetAttachParentActor` _asdestructible_actor))
    (`/Engine/EditorBlueprintResources/StandardMacros.IsValid` _returnvalue
      (:`Is Valid`
        (`self.K2_DestroyActor` _returnvalue))
      (:`Is Not Valid`
        _))
    (`self.K2_DestroyActor`)))

(event `self.OnProjectileFire`
  (`SceneComponent.SetHiddenInGame` (`self.Niagara`) false false)
  (`NiagaraFunctionLibrary.SpawnSystemAtLocation` "/Game/Effects/Particles/Explotion/NS_ky_explosion3.NS_ky_explosion3" (`self.K2_GetActorLocation`)))

(fn `UserConstructionScript`)