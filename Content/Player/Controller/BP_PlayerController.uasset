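; Player controller for the character lobby, relaying gamepad input to GM_Level according to the GameStatus held in GS_Level.
; In Spawn Character the interact buttons spawn a character, start the game or spawn an AI; in Customize Character they confirm, or cycle skin and character.
; A helper turns pressed keys into Next or Before by their index in the combined ChangeCharacter and ChangeSkin action mappings, so direction depends on mapping order.
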(event `self.ReceiveBeginPlay`
  (bind _asgm_level (cast `/Game/GameModes/GM_Level` (`GameplayStatics.GetGameMode`)))
  (set `self.GameMod` _asgm_level)
  (bind _asgs_level (cast `/Game/GameState/GS_Level` (`GameplayStatics.GetGameState`)))
  (set `self.GameState` _asgs_level))

(event `InputAction|InteractUI`
  (params (Key :type "Key Structure"))
  (:`Pressed`
    (bind _gamemod (`self.GameMod`)
      (:`then`
        (`self.InteractUISwitch` Key
          (:`A`
            (bind _gamestate (`self.GameState`)
              (:`then`
                (switch `EGameStatus` (`SFRMultiplayerGameState.GameStatus` _gamestate)
                  (:`SpawnCharacter`
                    (`SFRMultiplayerGameMode.SpawnNewCharacter` _gamemod self))
                  (:`CustomizeCharacter`
                    (`SFRMultiplayerGameMode.ConfirmCharacter` _gamemod))))
              (:`else`)))
          (:`B`
            (bind _gamestate_2 (`self.GameState`)
              (:`then`
                (switch `EGameStatus` (`SFRMultiplayerGameState.GameStatus` _gamestate_2)
                  (:`SpawnCharacter`
                    (`SFRMultiplayerGameMode.StartGame` _gamemod))))
              (:`else`)))
          (:`X`
            (bind _gamestate_3 (`self.GameState`)
              (:`then`
                (switch `EGameStatus` (`SFRMultiplayerGameState.GameStatus` _gamestate_3)
                  (:`SpawnCharacter`
                    (`SFRMultiplayerGameMode.SpawnAI` _gamemod null))))
              (:`else`)))))
      (:`else`))))

(event `InputAction|ChangeSkin`
  (params (Key :type "Key Structure"))
  (bind (_newparam _error) (`self.CastChangingInputToEnum` Key))
  (:`Pressed`
    (bind _gamemod (`self.GameMod`)
      (:`then`
        (bind _gamestate (`self.GameState`)
          (:`then`
            (if (not _error)
              (switch `EGameStatus` (`SFRMultiplayerGameState.GameStatus` _gamestate)
                (:`CustomizeCharacter`
                  (`SFRMultiplayerGameMode.ChangeSkin` _gamemod _newparam)))))
          (:`else`)))
      (:`else`))))

(event `InputAction|ChangeCharacter`
  (params (Key :type "Key Structure"))
  (bind (_newparam _error) (`self.CastChangingInputToEnum` Key))
  (:`Pressed`
    (bind _gamemod (`self.GameMod`)
      (:`then`
        (bind _gamestate (`self.GameState`)
          (:`then`
            (if (not _error)
              (switch `EGameStatus` (`SFRMultiplayerGameState.GameStatus` _gamestate)
                (:`CustomizeCharacter`
                  (`SFRMultiplayerGameMode.ChangeCharacter` _gamemod _newparam)))))
          (:`else`)))
      (:`else`))))

(fn `CastChangingInputToEnum`
  (params (InputPin :type "Key Structure" :default "None"))
  (returns (NewParam :type "EOrder Enum") (Error :type Boolean))
  (locals (ActionMap :type "Array of InputActionKeyMapping Structure"))
  (bind _output_get (set `local.ActionMap` (`InputSettings.GetActionMappingByName` (`InputSettings.GetInputSettings`) "ChangeCharacter")))
  (`KismetArrayLibrary.Array_Append` _output_get (`InputSettings.GetActionMappingByName` (`InputSettings.GetInputSettings`) "ChangeSkin"))
  (for (_array_element _array_index) (`local.ActionMap`)
    (if (== InputPin (`.Key` (break `InputActionKeyMapping` _array_element)))
      (switch `int` _array_index
        (:`0`
          _)
        (:`1`
          (return "Before" false))
        (:`2`
          _)
        (:`3`
          (return "Before" false)))
      (return "Next" false)))
  (return "Before" true))

(fn `UserConstructionScript`)