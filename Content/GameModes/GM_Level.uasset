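; Level game mode that runs a turn-based vehicle and skin selection for player controllers.
; Spawning places a character at the PlayerStart named by the current index and marks that controller's turn, with change events cycling its vehicle and skin.
; Finalizing possesses the vehicle, keeps the view on the shared selection camera, advances that camera and index, and hides HUD vehicle info.
; AI filling is an empty stub.
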(event `self.ReceiveBeginPlay`
  (set `self.GameModStatus` "NewEnumerator1")
  (bind _outactors (`GameplayStatics.GetAllActorsOfClass` "/Game/Blueprints/BP_ChooseCharacterCamera.BP_ChooseCharacterCamera_C"))
  (if (> (`KismetArrayLibrary.Array_Length` _outactors) 0)
    (bind _output_get (set `self.ChooseCharacterCamera` (`|GetArrayItem` _outactors)))
    (`PlayerController.SetViewTargetWithBlend` (`GameplayStatics.GetPlayerController` 0) _output_get 0.0 "VTBlend_Linear" 0.0 false)))

(event `SpawnPlayerCharacter`
  (params (ControllerID :type "/Game/Player/Controller/BP_PlayerController Object Reference"))
  (`self.ShowVehicleInfo` true
    (:`then`
      (set `self.GameModStatus` "NewEnumerator0")
      (bind _output_get (set `self.CurrnetController` ControllerID))
      (set `/Game/Player/Controller/BP_PlayerController.IsMyTurn` true _output_get)
      (bind _returnvalue (`|SpawnActorFromClass` "/Game/Player/Character/BP_PlayerCharacter.BP_PlayerCharacter_C" (`self.GetTransform` (`self.K2_FindPlayerStart` _output_get (`KismetStringLibrary.Conv_IntToString` (`self.CurrentVehicleIndex`)))) "AlwaysSpawn" "OverrideRootScale" null null))
      (set `self.CurrentVehicle` _returnvalue))))

(event `ChangeCharacterVehicle`
  (params (Next :type Boolean :default true))
  (bind _currentvehicle (`self.CurrentVehicle`))
  (if Next
    (`/Game/Player/Character/BP_PlayerCharacter.NextVehicle` _currentvehicle)
    (else
      (`/Game/Player/Character/BP_PlayerCharacter.PreviousVehicle` _currentvehicle))))

(event `FinalizePlayerCharacter`
  (bind _currnetcontroller (`self.CurrnetController`)
    (:`then`
      (set `/Game/Player/Controller/BP_PlayerController.HaveVehicle` true _currnetcontroller)
      (set `/Game/Player/Controller/BP_PlayerController.IsMyTurn` false _currnetcontroller)
      (bind _currentvehicle (`self.CurrentVehicle`)
        (:`then`
          (`Controller.Possess` _currnetcontroller _currentvehicle)
          (`PlayerController.SetViewTargetWithBlend` (`self.CurrnetController`) (`self.ChooseCharacterCamera`) 0.0 "VTBlend_Linear" 0.0 false)
          (`/Engine/EditorBlueprintResources/StandardMacros.IncrementInt` (`self.CurrentVehicleIndex`)
            (:`  `
              (set `self.CurrentVehicle` null)
              (`self.Next`)
              (set `self.GameModStatus` "NewEnumerator1")
              (`self.ShowVehicleInfo` false))))
        (:`else`)))
    (:`else`)))

(event `ChangeCharacterVehicleSkin`
  (params (Next :type Boolean :default true))
  (bind _currentvehicle (`self.CurrentVehicle`))
  (if Next
    (`/Game/Player/Character/BP_PlayerCharacter.NextSkin` _currentvehicle)
    (else
      (`/Game/Player/Character/BP_PlayerCharacter.PreviousSkin` _currentvehicle))))

(event `FillRestToAI`)

(event `Next`
  (`KismetSystemLibrary.PrintString` "Hello")
  (`/Game/Blueprints/BP_ChooseCharacterCamera.GoNext` (`self.ChooseCharacterCamera`)))

(fn `GetHud`
  (returns (ReturnValue :type "HUD Object Reference"))
  (return (`PlayerController.GetHUD` (`GameplayStatics.GetPlayerController` 0))))

(fn `GetMaxPlayer`
  (returns (ReturnValue :type Integer))
  (bind _outactors (`GameplayStatics.GetAllActorsOfClass` "/Script/Engine.PlayerStart"))
  (return (`KismetArrayLibrary.Array_Length` _outactors)))

(fn `UserConstructionScript`)